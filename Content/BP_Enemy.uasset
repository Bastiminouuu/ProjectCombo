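; Enemy Blueprint that turns to face a nearby Character and switches between idle and attack animations by proximity.
; Entering LookAtSphere stores the Character and starts a looping timer that interpolates yaw toward it, cleared on exit.
; The LootToAttack overlap volume toggles Attackornoattack, playing a non-looping combo attack on entry and idle on exit.
; Animations play directly on the mesh, and no damage is applied.
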(event `self.ReceiveBeginPlay`
  (if (`self.Attackornoattack`)
    (`SkeletalMeshComponent.PlayAnimation` (`self.Mesh`) "/Game/Sword_Animations/Animations/Sequence1/01_Idle/Idle_Seq.Idle_Seq" false)))

(event `self.LookAtSphere.OnComponentBeginOverlap`
  (params (OverlappedComponent :type "PrimitiveComponent Object Reference") (OtherActor :type "Actor Object Reference") (OtherComp :type "PrimitiveComponent Object Reference") (OtherBodyIndex :type Integer) (bFromSweep :type Boolean) (SweepResult :type "HitResult Structure (by ref)"))
  ;[0.1142 0.2793 1] Suivi du regard
  (bind _ascharacter (cast `Character` OtherActor))
  (set `self.CharRef` _ascharacter)
  (bind _returnvalue (`KismetSystemLibrary.K2_SetTimerDelegate` (delegate `Rotate`) 0.01 true))
  (set `self.Timer Handle` _returnvalue))

(event `self.LootToAttack.OnComponentBeginOverlap`
  (params (OverlappedComponent :type "PrimitiveComponent Object Reference") (OtherActor :type "Actor Object Reference") (OtherComp :type "PrimitiveComponent Object Reference") (OtherBodyIndex :type Integer) (bFromSweep :type Boolean) (SweepResult :type "HitResult Structure (by ref)"))
  ;[1 0.03409 0] Attack
  (if (not (`self.Attackornoattack`))
    (set `self.Attackornoattack` true)
    (`SkeletalMeshComponent.PlayAnimation` (`self.Mesh`) "/Game/Sword_Animations/Animations/Sequence1/02_Attack/05_Combo_Attack_Wave_05/Combo_Attack_Wave_05_02_Seq.Combo_Attack_Wave_05_02_Seq" false)))

(event `Rotate`
  (bind (_returnvalue_roll _returnvalue_pitch _returnvalue_yaw) (`KismetMathLibrary.BreakRotator` (`KismetMathLibrary.RInterpTo` (`self.K2_GetActorRotation`) (`KismetMathLibrary.FindLookAtRotation` (`self.K2_GetActorLocation`) (`self.K2_GetActorLocation` (`self.CharRef`))) (`GameplayStatics.GetWorldDeltaSeconds`) 5.0)))
  ;[0.1142 0.2793 1] Suivi du regard
  (`self.K2_SetActorRotation` (`KismetMathLibrary.MakeRotator` 0.0 0.0 _returnvalue_yaw)))

(event `self.LootToAttack.OnComponentEndOverlap`
  (params (OverlappedComponent :type "PrimitiveComponent Object Reference") (OtherActor :type "Actor Object Reference") (OtherComp :type "PrimitiveComponent Object Reference") (OtherBodyIndex :type Integer))
  ;[1 0.03409 0] Attack
  (if (`self.Attackornoattack`)
    (set `self.Attackornoattack` false)
    (`SkeletalMeshComponent.PlayAnimation` (`self.Mesh`) "/Game/Sword_Animations/Animations/Sequence1/01_Idle/Idle_Seq.Idle_Seq" false)))

(event `self.LookAtSphere.OnComponentEndOverlap`
  (params (OverlappedComponent :type "PrimitiveComponent Object Reference") (OtherActor :type "Actor Object Reference") (OtherComp :type "PrimitiveComponent Object Reference") (OtherBodyIndex :type Integer))
  ;[0.1142 0.2793 1] Suivi du regard
  (`KismetSystemLibrary.K2_ClearAndInvalidateTimerHandle` (`self.Timer Handle`)))

(fn `UserConstructionScript`)